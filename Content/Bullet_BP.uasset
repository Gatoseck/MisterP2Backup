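; Physics-driven bullet projectile that explodes on impact and breaks doors, windows and air vents.
; On BeginPlay it attaches a trail actor, plays a muzzle explosion, launches its capsule with a forward velocity impulse and self-destructs after two seconds.
; Hit spawns an explosion actor, particles and a colored Sound_Object, then detaches the trail before destroying itself.
; Overlap casts to each breakable type and applies radius damage to its destructible component.
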(event `self.ReceiveBeginPlay`
  (`self.AttachTrail`)
  (`self.InitialExplosion`)
  (`KismetSystemLibrary.Delay` 2.0)
  (`/Engine/EditorBlueprintResources/StandardMacros.IsValid` self
    (:`Is Valid`
      (`self.K2_DestroyActor`))))

(event `AttachTrail`
  (bind _returnvalue (`|SpawnActorFromClass` "/Game/Assets/Hero/Gun/Trail_BP.Trail_BP_C" (`KismetMathLibrary.MakeTransform` (`self.K2_GetActorLocation`)) "Undefined" "OverrideRootScale" null null null))
  (bind _output_get (set `self.Trail` _returnvalue))
  (`SceneComponent.K2_AttachToComponent` (`Actor.RootComponent` _output_get) (`self.Capsule`) "None" "SnapToTarget" "SnapToTarget" "SnapToTarget" true))

(event `InitialExplosion`
  (bind (_returnvalue_location _returnvalue_rotation) (`KismetMathLibrary.BreakTransform` (`self.GetTransform`)))
  (`GameplayStatics.SpawnEmitterAtLocation` "/Game/StarterContent/Particles/P_Explosion.P_Explosion" _returnvalue_location _returnvalue_rotation (`KismetMathLibrary.Conv_DoubleToVector` (`self.InitialExplosionSize`)))
  (`PrimitiveComponent.AddImpulse` (`self.Capsule`) (* (`self.GetActorForwardVector`) (`self.BulletSpeed`)) "None" true))

(event `self.ReceiveHit`
  (params (MyComp :type "PrimitiveComponent Object Reference") (Other :type "Actor Object Reference") (OtherComp :type "PrimitiveComponent Object Reference") (bSelfMoved :type Boolean) (HitLocation :type "Vector Structure") (HitNormal :type "Vector Structure") (NormalImpulse :type "Vector Structure") (Hit :type "HitResult Structure (by ref)"))
  (`|SpawnActorFromClass` "/Game/Assets/Hero/Gun/Explosion.Explosion_C" (`KismetMathLibrary.MakeTransform` HitLocation) "Undefined" "OverrideRootScale" null null)
  (`GameplayStatics.SpawnEmitterAtLocation` "/Game/StarterContent/Particles/P_Explosion.P_Explosion" HitLocation (struct) (`KismetMathLibrary.Conv_DoubleToVector` (`self.FinalExplosionSize`)))
  (bind _returnvalue (`|SpawnActorFromClass` "/Game/Assets/Sounds/Sound_Object.Sound_Object_C" (`KismetMathLibrary.MakeTransform` HitLocation) "Undefined" "OverrideRootScale" null null))
  (`/Game/Assets/Sounds/Sound_Object.Play 3D Sound` _returnvalue "/Game/StarterContent/Audio/Explosion01.Explosion01" 800.0 (struct :`R` 1.0 :`G` 0.042729 :`A` 1.0) 0.0 0.02 0.8 1.0 "/Game/Assets/Hero/Sounds/FootStepAttenuation.FootStepAttenuation")
  (`SceneComponent.K2_DetachFromComponent` (`Actor.RootComponent` (`self.Trail`)) "KeepWorld" "KeepWorld" "KeepWorld" true)
  (`self.K2_DestroyActor`))

(event `self.ReceiveActorBeginOverlap`
  (params (OtherActor :type "Actor Object Reference"))
  (bind _returnvalue (`self.K2_GetActorLocation` OtherActor))
  (bind _asdoor_bp (cast `/Game/Assets/Environment/Door/DoorBP` OtherActor)
    (:`then`
      (`DestructibleComponent.ApplyRadiusDamage` (`/Game/Assets/Environment/Door/DoorBP.Destructible` _asdoor_bp) 1000.0 _returnvalue 100.0 5.0 false))
    (:`CastFailed`
      (bind _aswindow_bp (cast `/Game/Assets/Environment/Window/Window_BP` OtherActor)
        (:`then`
          (`DestructibleComponent.ApplyRadiusDamage` (`/Game/Assets/Environment/Window/Window_BP.Destructible1` _aswindow_bp) 1000.0 _returnvalue 100.0 5.0 false))
        (:`CastFailed`
          (bind _asair_vent_bp (cast `/Game/Assets/Environment/AirVent/AirVent_BP` OtherActor))
          (`DestructibleComponent.ApplyRadiusDamage` (`/Game/Assets/Environment/AirVent/AirVent_BP.Destructible` _asair_vent_bp) 1000.0 _returnvalue 100.0 5.0 false))))))

(fn `UserConstructionScript`)