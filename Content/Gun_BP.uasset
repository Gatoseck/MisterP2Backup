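; Gun component that sets its parent static mesh to the gun model and handles firing.
; On Shoot, it spawns muzzle particles and a Bullet actor at the GunSocket, passing in its bullet, trail, damage, impulse and explosion settings.
; It also spawns a Sound_Object there to play the fire sound in 3D with color, intensity and size parameters, while separate final-sound values go to the bullet's explosion.
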(event `self.ReceiveBeginPlay`
  (bind _output_get (set `self.ParentMesh` (cast `StaticMeshComponent` (`|GetArrayItem` (`self.GetParentComponents`)) :!pure true)))
  (`StaticMeshComponent.SetStaticMesh` _output_get (`self.GunMesh`)))

(event `Shoot`
  (bind _returnvalue (`self.GetSocketTransform` (`self.ParentMesh`) "GunSocket" "RTS_World"))
  (`GameplayStatics.SpawnEmitterAtLocation` (`self.FireParticles`) (`self.GetSocketLocation` (`self.ParentMesh`) "GunSocket") (struct) (`KismetMathLibrary.Conv_DoubleToVector` (`self.FireSize`)))
  (`|SpawnActorFromClass` "/Game/Assets/Hero/Gun/Bullet.Bullet_C" _returnvalue "Undefined" "OverrideRootScale" null (`self.BulletSpeed`) (`self.BulletSize`) (`self.TrailParticles`) (`self.ExplosiveDamage`) (`self.ExplosiveDamageSize`) (`self.ExplosionSize`) (`self.ExplosionParticles`) (`self.ExplosionSound`) (`self.SoundIntensityFinal`) (`self.SoundSizeMultiplierFinal`) (`self.SoundColorFinal`) (`self.BulletDamage`) (`self.ImpulseStrengh`) null)
  (bind _returnvalue_2 (`|SpawnActorFromClass` "/Game/Assets/Sounds/Sound_Object.Sound_Object_C" _returnvalue "Undefined" "OverrideRootScale" null null))
  (`/Game/Assets/Sounds/Sound_Object.Play 3D Sound` _returnvalue_2 (`self.FireSound`) (`self.SoundIntensity`) (`self.SoundColor`) 0.0 (`self.SoundSizeMultiplier`) 0.8 1.0 "/Game/Assets/Hero/Sounds/FootStepAttenuation.FootStepAttenuation"))