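; Door Blueprint that starts closed when its KeyID is nonzero and open otherwise.
; BeginPlay passes that state to the OpenCloseDoor event, which disables Box collision when open and enables query and physics collision when closed.
; Unconnected leftover nodes would constrain a static mesh to a destructible child actor and toggle that destructible's PhysicsBody collision response, but they never run.
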(event `self.ReceiveBeginPlay`
  (if (!= (`self.KeyID`) 0)
    (`self.OpenCloseDoor` false)
    (else
      (`self.OpenCloseDoor` true))))

(event `OpenCloseDoor`
  (params (`Open?` :type Boolean))
  (bind _box (`self.Box`))
  (if `Open?`
    (`PrimitiveComponent.SetCollisionEnabled` _box "NoCollision")
    (else
      (`PrimitiveComponent.SetCollisionEnabled` _box "QueryAndPhysics"))))

(fn `UserConstructionScript`)